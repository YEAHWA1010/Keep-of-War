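; Showcase archer character that automatically cycles clothing swatches and swaps between bow and axe on looping delays, with keys for manual changes.
; Construction creates dynamic material instances on three mesh slots, which receive the selected swatch texture.
; Weapon updates toggle component visibility and set the AnimBP's left-arm animation.
; Left click plays per-weapon combo montages, while separate events animate the bow and spawn arrows; AutoRotation is an empty stub.
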(event `self.ReceiveBeginPlay`
  ;[1 1 1] Begin Play and Set AnimBP
  (`|ExecutionSequence`
    (:`then_1`
      (`self.Change Swatch` :!label _label)
      (`KismetSystemLibrary.Delay` 2.0)
      (goto _label))
    (:`then_2`
      (`/Engine/EditorBlueprintResources/StandardMacros.FlipFlop` :!label _label_2
        (:`A`
          (set `self.Weapon` "NewEnumerator0"))
        (:`B`
          (set `self.Weapon` "NewEnumerator1")))
      (`self.Update Weapon`)
      (`KismetSystemLibrary.Delay` 3.0)
      (goto _label_2))))

(event `Set Dynamic Material Instance`
  (bind _mesh (`self.Mesh`))
  ;[1 1 1] Set Dynamic Material Instance
  (`|ExecutionSequence`
    (:`then_0`
      (bind _returnvalue (`PrimitiveComponent.CreateDynamicMaterialInstance` _mesh 0 "/Game/RK_Fantasy_Archer/Materials/clothing_one_Mat_Inst.clothing_one_Mat_Inst" "None"))
      (set `self.Element0` _returnvalue))
    (:`then_1`
      (bind _returnvalue_2 (`PrimitiveComponent.CreateDynamicMaterialInstance` _mesh 6 "/Game/RK_Fantasy_Archer/Materials/clothing_one_Mat_Inst.clothing_one_Mat_Inst" "None"))
      (set `self.Element6` _returnvalue_2))
    (:`then_2`
      (bind _returnvalue_3 (`PrimitiveComponent.CreateDynamicMaterialInstance` _mesh 7 "/Game/RK_Fantasy_Archer/Materials/clothing_one_Mat_Inst.clothing_one_Mat_Inst" "None"))
      (set `self.Element7` _returnvalue_3))
    (:`then_3`
      (`self.Check and Set new Swatches`))))

(event `Update Weapon`
  (bind _animbp (`self.AnimBP`))
  ;[1 1 1] Update Weapon
  (bind _asfantasy_archer_anim_bp (cast `/Game/RK_Fantasy_Archer/Animations/BlendSpace/Fantasy_Archer_AnimBP` (`SkeletalMeshComponent.GetAnimInstance` (`self.Mesh`))))
  (set `self.AnimBP` _asfantasy_archer_anim_bp)
  (switch `/Game/RK_Fantasy_Archer/Enums/Weapon` (`self.Weapon`)
    (:`NewEnumerator0`
      (`SceneComponent.SetVisibility` (`self.Bow`) true false)
      (`SceneComponent.SetVisibility` (`self.Axe`) false false)
      (set `/Game/RK_Fantasy_Archer/Animations/BlendSpace/Fantasy_Archer_AnimBP.Left Arm Animation` "/Game/RK_Fantasy_Archer/Animations/Bow_Attacks/Bow_Left_Arm.Bow_Left_Arm" _animbp))
    (:`NewEnumerator1`
      (`SceneComponent.SetVisibility` (`self.Bow`) false false)
      (`SceneComponent.SetVisibility` (`self.Axe`) true false)
      (set `/Game/RK_Fantasy_Archer/Animations/BlendSpace/Fantasy_Archer_AnimBP.Left Arm Animation` null _animbp))))

(event `Key|LeftMouseButton`
  (params (Key :type "Key Structure"))
  ;[1 1 1] Attack Events
  (:`Pressed`
    (if (not (`AnimInstance.Montage_IsPlaying` (`SkeletalMeshComponent.GetAnimInstance` (`self.Mesh`)) null))
      (switch `/Game/RK_Fantasy_Archer/Enums/Weapon` (`self.Weapon`)
        (:`NewEnumerator0`
          (switch `int` (`self.Attack_Combo`)
            (:`0`
              (set `self.Attack_Combo` 1)
              (`self.PlayAnimMontage` "/Game/RK_Fantasy_Archer/Animations/Bow_Attacks/Attack_Bow_1_Montage.Attack_Bow_1_Montage"))
            (:`1`
              (set `self.Attack_Combo` 2)
              (`self.PlayAnimMontage` "/Game/RK_Fantasy_Archer/Animations/Bow_Attacks/Attack_Bow_2_Montage.Attack_Bow_2_Montage"))
            (:`2`
              (set `self.Attack_Combo` 3)
              (`self.PlayAnimMontage` "/Game/RK_Fantasy_Archer/Animations/Bow_Attacks/Attack_Bow_3_Montage.Attack_Bow_3_Montage"))
            (:`3`
              (set `self.Attack_Combo` 0)
              (`self.PlayAnimMontage` "/Game/RK_Fantasy_Archer/Animations/Bow_Attacks/Attack_Bow_4_Montage.Attack_Bow_4_Montage"))))
        (:`NewEnumerator1`
          (switch `int` (`self.Attack_Combo`)
            (:`0`
              (set `self.Attack_Combo` 1)
              (`self.PlayAnimMontage` "/Game/RK_Fantasy_Archer/Animations/Axe_Attacks/Attack_Axe1_Montage.Attack_Axe1_Montage"))
            (:`1`
              (set `self.Attack_Combo` 2)
              (`self.PlayAnimMontage` "/Game/RK_Fantasy_Archer/Animations/Axe_Attacks/Attack_Axe2_Montage.Attack_Axe2_Montage"))
            (:`2`
              (set `self.Attack_Combo` 0)
              (`self.PlayAnimMontage` "/Game/RK_Fantasy_Archer/Animations/Axe_Attacks/Attack_Axe3_Montage.Attack_Axe3_Montage"))))))))

(event `Check and Set new Swatches`
  ;[1 1 1] Set Swatches
  (switch `/Game/RK_Fantasy_Archer/Enums/Swatches` (`self.Swatch`)
    (:`NewEnumerator0`
      (set `self.Current Swatch` "/Game/RK_Fantasy_Archer/Textures/swatches/blue_dk.blue_dk"))
    (:`NewEnumerator1`
      (set `self.Current Swatch` "/Game/RK_Fantasy_Archer/Textures/swatches/blue_lt.blue_lt"))
    (:`NewEnumerator2`
      (set `self.Current Swatch` "/Game/RK_Fantasy_Archer/Textures/swatches/brown_mid.brown_mid"))
    (:`NewEnumerator3`
      (set `self.Current Swatch` "/Game/RK_Fantasy_Archer/Textures/swatches/checks.checks"))
    (:`NewEnumerator4`
      (set `self.Current Swatch` "/Game/RK_Fantasy_Archer/Textures/swatches/checks2.checks2"))
    (:`NewEnumerator5`
      (set `self.Current Swatch` "/Game/RK_Fantasy_Archer/Textures/swatches/exotic.exotic"))
    (:`NewEnumerator6`
      (set `self.Current Swatch` "/Game/RK_Fantasy_Archer/Textures/swatches/green_camo.green_camo"))
    (:`NewEnumerator7`
      (set `self.Current Swatch` "/Game/RK_Fantasy_Archer/Textures/swatches/green_lt.green_lt"))
    (:`NewEnumerator8`
      (set `self.Current Swatch` "/Game/RK_Fantasy_Archer/Textures/swatches/green_camo.green_camo"))
    (:`NewEnumerator9`
      (set `self.Current Swatch` "/Game/RK_Fantasy_Archer/Textures/swatches/grey_dk.grey_dk"))
    (:`NewEnumerator10`
      (set `self.Current Swatch` "/Game/RK_Fantasy_Archer/Textures/swatches/grey_mid.grey_mid"))
    (:`NewEnumerator11`
      (set `self.Current Swatch` "/Game/RK_Fantasy_Archer/Textures/swatches/olive.olive"))
    (:`NewEnumerator12`
      (set `self.Current Swatch` "/Game/RK_Fantasy_Archer/Textures/swatches/orange.orange"))
    (:`NewEnumerator13`
      (set `self.Current Swatch` "/Game/RK_Fantasy_Archer/Textures/swatches/pattern_mid.pattern_mid"))
    (:`NewEnumerator14`
      (set `self.Current Swatch` "/Game/RK_Fantasy_Archer/Textures/swatches/plaid_lt.plaid_lt"))
    (:`NewEnumerator15`
      (set `self.Current Swatch` "/Game/RK_Fantasy_Archer/Textures/swatches/purple_mid.purple_mid"))
    (:`NewEnumerator16`
      (set `self.Current Swatch` "/Game/RK_Fantasy_Archer/Textures/swatches/star.star")))
  (`MaterialInstanceDynamic.SetTextureParameterValue` (`self.Element0`) "Swatch" (`self.Current Swatch`))
  (`MaterialInstanceDynamic.SetTextureParameterValue` (`self.Element6`) "Swatch" (`self.Current Swatch`))
  (`MaterialInstanceDynamic.SetTextureParameterValue` (`self.Element7`) "Swatch" (`self.Current Swatch`)))

(event `Bow Shot Animation`
  ;[1 1 1] Bow Events
  (`SkeletalMeshComponent.PlayAnimation` (`self.Bow`) "/Game/RK_Fantasy_Archer/Animations/Bow_Attacks/Bow_Shot_Animation_Anim.Bow_Shot_Animation_Anim" false))

(event `Bow Shot Animation End`
  ;[1 1 1] Bow Events
  (`SkeletalMeshComponent.PlayAnimation` (`self.Bow`) "/Game/RK_Fantasy_Archer/Animations/Bow_Attacks/Bow_Shot_Animation_END.Bow_Shot_Animation_END" false))

(event `Spawn Arrow`
  ;[1 1 1] Bow Events
  (`|SpawnActorFromClass` "/Game/RK_Fantasy_Archer/Blueprints/BP_Archer_Arrow_Projectile.BP_Archer_Arrow_Projectile_C" (`KismetMathLibrary.MakeTransform` (`SceneComponent.GetSocketLocation` (`self.Mesh`) "Hand_R") (`self.K2_GetActorRotation`)) "Undefined" "MultiplyWithRoot" null null))

(event `Change Swatch`
  (bind _swatch (`self.Swatch`))
  ;[1 1 1] Change Swatch Color Input
  (if (< _swatch 16) :!label _label
    (set `self.Swatch` (cast `/Game/RK_Fantasy_Archer/Enums/Swatches` (+ _swatch 1)))
    (else
      (set `self.Swatch` "NewEnumerator0")))
  (`self.Check and Set new Swatches`))

(event `Key|One`
  (params (Key :type "Key Structure"))
  ;[1 1 1] Change Swatch Color Input
  (:`Pressed`
    (goto _label)))

(event `Key|Two`
  (params (Key :type "Key Structure"))
  ;[1 1 1] Change Weapon
  (:`Pressed`
    (switch `/Game/RK_Fantasy_Archer/Enums/Weapon` (`self.Weapon`)
      (:`NewEnumerator0`
        (set `self.Weapon` "NewEnumerator1"))
      (:`NewEnumerator1`
        (set `self.Weapon` "NewEnumerator0")))
    (`self.Update Weapon`)))

(fn `UserConstructionScript`
  (`self.Set Dynamic Material Instance`)
  (`self.Update Weapon`))