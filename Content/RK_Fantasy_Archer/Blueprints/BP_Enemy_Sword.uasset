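; BP_Enemy_Sword is a modular Fantasy Archer character Blueprint with selectable clothing swatches and an optional hood and face mask.
; Its construction script creates dynamic materials for body, hood and mask, then sets their "Swatch" texture from an enum.
; Hood and mask follow the main mesh through leader pose, with visibility set by the Clothing option.
; Leftover logic for cycling swatch, clothing and bow/axe never runs, and no combat logic is present.
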(event `Set Dynamic Material Instance`
  ;[1 1 1] Set Dynamic Material Instance
  (`|ExecutionSequence`
    (:`then_0`
      (bind _returnvalue (`PrimitiveComponent.CreateDynamicMaterialInstance` (`self.Mesh`) 0 "/Game/RK_Fantasy_Archer/Materials/clothing_one_Mat_Inst.clothing_one_Mat_Inst" "None"))
      (set `self.Element0` _returnvalue))
    (:`then_1`
      (bind _returnvalue_2 (`PrimitiveComponent.CreateDynamicMaterialInstance` (`self.Hood`) 0 "/Game/RK_Fantasy_Archer/Materials/clothing_one_Mat_Inst.clothing_one_Mat_Inst" "None"))
      (set `self.Element6` _returnvalue_2))
    (:`then_2`
      (bind _returnvalue_3 (`PrimitiveComponent.CreateDynamicMaterialInstance` (`self.Face_Mask`) 0 "/Game/RK_Fantasy_Archer/Materials/clothing_one_Mat_Inst.clothing_one_Mat_Inst" "None"))
      (set `self.Element7` _returnvalue_3))
    (:`then_3`
      (`self.Check and Set new Swatches`))))

(event `Check and Set new Swatches`
  ;[1 1 1] Set Swatches
  (switch `/Game/RK_Fantasy_Archer/Enums/Swatches` (`self.Swatch`)
    (:`NewEnumerator0`
      (set `self.Current Swatch` "/Game/RK_Fantasy_Archer/Textures/swatches/blue_dk.blue_dk"))
    (:`NewEnumerator1`
      (set `self.Current Swatch` "/Game/RK_Fantasy_Archer/Textures/swatches/blue_lt.blue_lt"))
    (:`NewEnumerator2`
      (set `self.Current Swatch` "/Game/RK_Fantasy_Archer/Textures/swatches/brown_mid.brown_mid"))
    (:`NewEnumerator3`
      (set `self.Current Swatch` "/Game/RK_Fantasy_Archer/Textures/swatches/checks.checks"))
    (:`NewEnumerator4`
      (set `self.Current Swatch` "/Game/RK_Fantasy_Archer/Textures/swatches/checks2.checks2"))
    (:`NewEnumerator5`
      (set `self.Current Swatch` "/Game/RK_Fantasy_Archer/Textures/swatches/exotic.exotic"))
    (:`NewEnumerator6`
      (set `self.Current Swatch` "/Game/RK_Fantasy_Archer/Textures/swatches/green_camo.green_camo"))
    (:`NewEnumerator7`
      (set `self.Current Swatch` "/Game/RK_Fantasy_Archer/Textures/swatches/green_lt.green_lt"))
    (:`NewEnumerator8`
      (set `self.Current Swatch` "/Game/RK_Fantasy_Archer/Textures/swatches/green_camo.green_camo"))
    (:`NewEnumerator9`
      (set `self.Current Swatch` "/Game/RK_Fantasy_Archer/Textures/swatches/grey_dk.grey_dk"))
    (:`NewEnumerator10`
      (set `self.Current Swatch` "/Game/RK_Fantasy_Archer/Textures/swatches/grey_mid.grey_mid"))
    (:`NewEnumerator11`
      (set `self.Current Swatch` "/Game/RK_Fantasy_Archer/Textures/swatches/olive.olive"))
    (:`NewEnumerator12`
      (set `self.Current Swatch` "/Game/RK_Fantasy_Archer/Textures/swatches/orange.orange"))
    (:`NewEnumerator13`
      (set `self.Current Swatch` "/Game/RK_Fantasy_Archer/Textures/swatches/pattern_mid.pattern_mid"))
    (:`NewEnumerator14`
      (set `self.Current Swatch` "/Game/RK_Fantasy_Archer/Textures/swatches/plaid_lt.plaid_lt"))
    (:`NewEnumerator15`
      (set `self.Current Swatch` "/Game/RK_Fantasy_Archer/Textures/swatches/purple_mid.purple_mid"))
    (:`NewEnumerator16`
      (set `self.Current Swatch` "/Game/RK_Fantasy_Archer/Textures/swatches/star.star")))
  (`MaterialInstanceDynamic.SetTextureParameterValue` (`self.Element0`) "Swatch" (`self.Current Swatch`))
  (`MaterialInstanceDynamic.SetTextureParameterValue` (`self.Element6`) "Swatch" (`self.Current Swatch`))
  (`MaterialInstanceDynamic.SetTextureParameterValue` (`self.Element7`) "Swatch" (`self.Current Swatch`)))

(event `Update Clothing`
  ;[1 1 1] Update Clothing
  (switch `/Game/RK_Fantasy_Archer/Enums/Clothing` (`self.Clothing`)
    (:`NewEnumerator4`
      (`SceneComponent.SetVisibility` (`self.Face_Mask`) true false)
      (`SceneComponent.SetVisibility` (`self.Hood`) true false))
    (:`NewEnumerator5`
      (`SceneComponent.SetVisibility` (`self.Face_Mask`) false false)
      (`SceneComponent.SetVisibility` (`self.Hood`) false false))))

(event `Key|One`
  (params (Key :type "Key Structure"))
  ;[1 1 1] Change Swatch Color Input
)

(event `Key|Two`
  (params (Key :type "Key Structure"))
  ;[1 1 1] Change Weapons
)

(event `Key|Three`
  (params (Key :type "Key Structure"))
  ;[1 1 1] Update Clothing
)

(fn `UserConstructionScript`
  (`self.Set Dynamic Material Instance`)
  (`SkinnedMeshComponent.SetLeaderPoseComponent` (`self.Hood`) (`self.Mesh`) false false)
  (`SkinnedMeshComponent.SetLeaderPoseComponent` (`self.Face_Mask`) (`self.Mesh`) false false)
  (`self.Update Clothing`))